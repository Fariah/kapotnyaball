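; Ball actor whose position is driven by the server and which triggers its own respawn.
; Every tick the authority multicasts the ball's transform, and receivers set it directly without sweep or teleport.
; On destruction the authority asks the GameplayGM game mode to respawn the ball.
; The transform OnRep function is empty, so syncing relies on the multicast.
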(event `MulticastPosition`
  (params (NewTransform :type "Transform Structure (by ref)"))
  ;[1 1 1] Multicast ball postion
  (`self.K2_SetActorTransform` NewTransform))

(event `self.ReceiveTick`
  (params (DeltaSeconds :type "Float (single-precision)"))
  ;[1 1 1] Multicast ball postion
  (`/Engine/EditorBlueprintResources/ActorMacros.Switch Has Authority`
    (:`Authority`
      (`self.MulticastPosition` (`self.GetTransform`)))))

(event `self.ReceiveDestroyed`
  ;[1 1 1] Respawn ball
  (`/Engine/EditorBlueprintResources/ActorMacros.Switch Has Authority`
    (:`Authority`
      (bind _asgameplay_gm (cast `/Game/Blueprints/Gameplay/GameplayGM` (`GameplayStatics.GetGameMode`)))
      (`/Game/Blueprints/Gameplay/GameplayGM.respawnBall` _asgameplay_gm)
      (`KismetSystemLibrary.PrintString` "Ball respawned" true true (struct :`G` 0.536458 :`B` 0.047946 :`A` 1.0) 5.0))))

(fn `OnRep_transform`)

(fn `UserConstructionScript`)