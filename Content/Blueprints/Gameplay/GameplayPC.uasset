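; Player controller for gameplay that loads the player's saved settings and requests their chosen ball character from the game mode.
; On BeginPlay the local controller clears widgets, reads the save slot and hands the settings to PassCharactertoServer, which calls RespawnPlayer on GameplayGM.
; Holding Tab shows a score widget, created fresh on each press and removed on release.
; A mouse cursor toggle exists but is unconnected.
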(event `Key|Tab`
  (params (Key :type "Key Structure"))
  (bind _scorewidgget (`self.ScoreWidgget`))
  ;[1 1 1] Score Event
  (:`Pressed`
    (bind _returnvalue (`|CreateWidget` "/Game/UI/AllLevels/W_Score.W_Score_C"))
    (bind _output_get (set `self.ScoreWidgget` _returnvalue))
    (`UserWidget.AddToPlayerScreen` _output_get 0))
  (:`Released`
    (`/Engine/EditorBlueprintResources/StandardMacros.IsValid` _scorewidgget
      (:`Is Valid`
        (`Widget.RemoveFromParent` _scorewidgget)))))

(event `self.ReceiveBeginPlay`
  ;[1 1 1] Load Player Info and pass to server side
  (if (`self.IsLocalController`)
    (`WidgetLayoutLibrary.RemoveAllWidgets`)
    (`self.LoadGame`)
    (`self.PassCharactertoServer` (`self.PlayerSettings`))))

(event `PassCharactertoServer`
  (params (PlayerSettingsInfo :type "/Game/Blueprints/AllLevels/PlayerInfo Structure"))
  ;[1 1 1] Passes character info
  (set `self.PlayerSettings` PlayerSettingsInfo)
  (bind _asgameplay_gm (cast `/Game/Blueprints/Gameplay/GameplayGM` (`GameplayStatics.GetGameMode`)))
  (`/Game/Blueprints/Gameplay/GameplayGM.RespawnPlayer` _asgameplay_gm self (`.MyPlayerBall_25_228EAD3B4EAA9E2BC00192BF52025C9F` (break `/Game/Blueprints/AllLevels/PlayerInfo` (`self.PlayerSettings`)))))

(event `Key|T`
  (params (Key :type "Key Structure"))
  ;[1 1 1] T to type
)

(fn `LoadGame`
  (bind _returnvalue (`GameplayStatics.LoadGameFromSlot` (`self.PlayerSettingsSave`)))
  (bind _asplayer_save_game (cast `/Game/Blueprints/AllLevels/PlayerSaveGame` _returnvalue))
  (set `self.PlayerSettings` (`/Game/Blueprints/AllLevels/PlayerSaveGame.S_PlayerInfo` _asplayer_save_game)))

(fn `UserConstructionScript`)