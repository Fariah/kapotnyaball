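; Blue-side goal trigger box that awards a point to the red team when a ball enters it.
; On overlap, the authority checks the actor's tag, runs the score event to update BallGameStateBase and print a message, then destroys the ball.
; A separate helper, not called here, writes a value to every TextRenderActor with a matching color tag.
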(event `ServerScoreBlue`
  (bind _asball_game_state_base (cast `/Game/Blueprints/Gameplay/BallGameStateBase` (`GameplayStatics.GetGameState`)))
  (`/Game/Blueprints/Gameplay/BallGameStateBase.SetTeamScore_Event` _asball_game_state_base "red")
  (`KismetSystemLibrary.PrintString` "+1 to red team" true true (struct :`R` 0.65625 :`A` 1.0) 3.0))

(event `self.ReceiveActorBeginOverlap`
  (params (OtherActor :type "Actor Object Reference"))
  (`/Engine/EditorBlueprintResources/ActorMacros.Switch Has Authority`
    (:`Authority`
      (set `self.Actor` OtherActor)
      (if (`self.ActorHasTag` OtherActor (`self.TagNameBall`))
        (`self.ServerScoreBlue`)
        (`self.K2_DestroyActor` (`self.Actor`))))))

(fn `SetTextToActor`
  (params (Value :type Integer))
  (bind _outactors (`GameplayStatics.GetAllActorsOfClass` "/Script/Engine.TextRenderActor"))
  (for _array_element _outactors
    (if (`self.ActorHasTag` _array_element (`self.TagColor`))
      (`TextRenderComponent.K2_SetText` (`TextRenderActor.TextRender` _array_element) (`KismetTextLibrary.Conv_IntToText` Value)))))

(fn `UserConstructionScript`)