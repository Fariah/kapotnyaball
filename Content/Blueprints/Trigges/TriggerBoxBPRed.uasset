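; Red goal trigger box that awards a point to the blue team when a ball enters it.
; On overlap with authority, an actor carrying the ball tag fires ServerScoreRed, which calls SetTeamScoreEvent on BallGameStateBase, then the ball is destroyed.
; A separate SetTextToActor function writes a given score to color-tagged TextRenderActors, but nothing in this graph calls it.
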(event `ServerScoreRed`
  (bind _asball_game_state_base (cast `/Game/Blueprints/Gameplay/BallGameStateBase` (`GameplayStatics.GetGameState`)))
  (`/Game/Blueprints/Gameplay/BallGameStateBase.SetTeamScore_Event` _asball_game_state_base "blue")
  (`KismetSystemLibrary.PrintString` "+1 to blue team" true true (struct :`G` 0.015459 :`B` 0.484375 :`A` 1.0) 3.0))

(event `self.ReceiveActorBeginOverlap`
  (params (OtherActor :type "Actor Object Reference"))
  (`/Engine/EditorBlueprintResources/ActorMacros.Switch Has Authority`
    (:`Authority`
      (set `self.Actor` OtherActor)
      (if (`self.ActorHasTag` OtherActor (`self.BallTag`))
        (`self.ServerScoreRed`)
        (`self.K2_DestroyActor` (`self.Actor`))))))

(fn `SetTextToActor`
  (params (Score :type Integer))
  (bind _outactors (`GameplayStatics.GetAllActorsOfClass` "/Script/Engine.TextRenderActor"))
  (for _array_element _outactors
    (if (`self.ActorHasTag` _array_element (`self.TagColor`))
      (`TextRenderComponent.K2_SetText` (`TextRenderActor.TextRender` _array_element) (`KismetTextLibrary.Conv_IntToText` Score)))))

(fn `UserConstructionScript`)